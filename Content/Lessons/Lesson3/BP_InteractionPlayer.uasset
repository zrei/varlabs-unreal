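; BP_InteractionPlayer is a VR player that aims by gaze and scores points by interacting with actors.
; Every Tick, a camera-forward line trace places a billboard reticle at the hit point, or at maximum range.
; The Act input repeats the trace and adds the hit actor's InteractMessage return value to Score.
; It then updates the Scoreboard found at BeginPlay and spawns BP_ScoreAddition with a chime at the hit.
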(event `self.ReceiveBeginPlay`
  (bind _outactors (`GameplayStatics.GetAllActorsOfClass` "/Game/Lessons/Lesson3/BP_Scoreboard.BP_Scoreboard_C"))
  (set `self.Scoreboard` (`|GetArrayItem` _outactors)))

(event `self.ReceiveTick`
  (params (DeltaSeconds :type "Float (single-precision)"))
  (bind _materialbillboard (`self.MaterialBillboard`))
  (bind (_location _forward_vector) (`/Game/Blueprints/Utility/VARlabsVRUtilityFunctions.Get Player VR Camera Properties`))
  (bind _returnvalue (+ (* _forward_vector 10000.0) _location))
  (bind (_outhit _returnvalue_2) (`KismetSystemLibrary.LineTraceSingle` _location _returnvalue "TraceTypeQuery1"))
  (if _returnvalue_2
    (`SceneComponent.K2_SetWorldLocation` _materialbillboard (`.Location` (`GameplayStatics.BreakHitResult` _outhit)) false false)
    (else
      (`SceneComponent.K2_SetWorldLocation` _materialbillboard _returnvalue false false))))

(event `InputAction|Act`
  (params (Key :type "Key Structure"))
  (:`Pressed`
    (`KismetSystemLibrary.PrintString` "Firing")
    (bind (_location _forward_vector) (`/Game/Blueprints/Utility/VARlabsVRUtilityFunctions.Get Player VR Camera Properties`))
    (bind (_outhit _returnvalue) (`KismetSystemLibrary.LineTraceSingle` :`Start` _location :`End` (+ (* _forward_vector 10000.0) _location) :`TraceChannel` "TraceTypeQuery1" :`DrawDebugType` "ForDuration"))
    (if _returnvalue
      (bind (_bblockinghit _binitialoverlap _time _distance _location_2 _impactpoint _normal _impactnormal _physmat _hitactor) (`GameplayStatics.BreakHitResult` _outhit))
      (bind _score (message `/Game/Lessons/Lesson3/BPI_Interaction.Interact` _hitactor))
      (bind _output_get (set `self.Score` (+ (`self.Score`) _score)))
      (`KismetSystemLibrary.PrintString` (`KismetStringLibrary.Conv_IntToString` _output_get))
      (`/Game/Lessons/Lesson3/BP_Scoreboard.UpdateScore` (`self.Scoreboard`) _output_get)
      (`|SpawnActorFromClass` "/Game/Lessons/Lesson3/BP_ScoreAddition.BP_ScoreAddition_C" (`KismetMathLibrary.MakeTransform` _location_2) "Undefined" "OverrideRootScale" null 0 20.0 null)
      (`GameplayStatics.SpawnSoundAtLocation` "/Game/Audio/SoundWaves/Effect/SW_Chime_1.SW_Chime_1" _location_2 (struct) 1.0 1.0 0.0 null null))))

(fn `UserConstructionScript`)