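; Game manager for a multi-level falling-fruit score game, running timed rounds with per-level high scores.
; StartGame loads that level's settings, resets state, hides via VisibilityManager and spawns a blocker on the last level.
; Tick advances timers, spawning bombs or weighted-random fruit between two bound actors at set intervals until a cutoff.
; When time expires, EndGame records the high score, restores visibility, shows result text with sound and removes the blocker.
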(event `self.ReceiveBeginPlay`
  (bind _outactors (`GameplayStatics.GetAllActorsOfClass` "/Game/Lessons/Lesson3/miniProject3/Blueprints/BP_VisibilityManager.BP_VisibilityManager_C"))
  (set `self.visibilityManager` (`|GetArrayItem` _outactors)))

(event `self.ReceiveTick`
  (params (DeltaSeconds :type "Float (single-precision)"))
  (if (`self.inGame`)
    (`self.UpdateTimers` DeltaSeconds)
    (`self.CheckToSpawn`)
    (`self.CheckGameOver`)))

(fn `CheckGameOver`
  (if (>= (`self.currGameTime`) (`self.gameTime`))
    (`self.EndGame`)))

(fn `CheckToSpawn`
  (if (< (`self.currGameTime`) (`self.spawnTime`))
    (if (>= (`self.intervalTimer`) (`.SpawnInterval_9_0D1334314143EE0FBEB05091E680C5D3` (break `/Game/Lessons/Lesson3/miniProject3/Blueprints/Structs/S_DifficultySettings` (`self.currGameDetails`))))
      (bind _spawnlocation (`self.ChooseSpawnPoint`))
      (`self.SpawnObject` _spawnlocation)
      (set `self.intervalTimer` 0.0))))

(fn `ChooseFruit`
  (returns (FruitType :type "/Game/Lessons/Lesson3/miniProject3/Blueprints/E_FruitTypes Enum"))
  (locals (randomFloat :type "Float (double-precision)"))
  (bind (_watermelonspawnchance _orangespawnchance) (break `/Game/Lessons/Lesson3/miniProject3/Blueprints/Structs/S_FruitSpawnChance` (`self.spawnChances`)))
  (bind _output_get (set `local.randomFloat` (`KismetMathLibrary.RandomFloatInRange` 0.0 1.0)))
  (if (<= _output_get _watermelonspawnchance)
    (return "NewEnumerator0")
    (elif (<= _output_get (+ _watermelonspawnchance _orangespawnchance))
      (return "NewEnumerator1")
      (else
        (return "NewEnumerator2")))))

(fn `ChooseSpawnPoint`
  (returns (SpawnLocation :type "Vector Structure"))
  (return (`KismetMathLibrary.MakeVector` (.x (`self.leftSpawnBound`)) (`KismetMathLibrary.RandomFloatInRange` (.y (`self.leftSpawnBound`)) (.y (`self.rightSpawnBound`))) (.z (`self.leftSpawnBound`)))))

(fn `DestroyObstacles`
  (bind _obstacleinstance (`self.obstacleInstance`))
  (if (`KismetSystemLibrary.IsValid` _obstacleinstance)
    (`self.K2_DestroyActor` _obstacleinstance))
  (set `self.obstacleInstance` null))

(fn `EndGame`
  (bind _highscoreupdated (`self.UpdateHighScore`))
  (set `self.inGame` false)
  (`KismetSystemLibrary.PrintString` "End Game")
  (`/Game/Lessons/Lesson3/miniProject3/Blueprints/BP_VisibilityManager.SetVisible` (`self.visibilityManager`))
  (`/Game/Lessons/Lesson3/miniProject3/Blueprints/BP_Text.Hide` (`self.scoreText`))
  (`self.UpdateGameEndStatus` _highscoreupdated)
  (`self.DestroyObstacles`))

(fn `GetHighScore`
  (params (Level :type Integer))
  (returns (HighScore :type Integer))
  (return (`|GetArrayItem` (`self.HighScores`) Level)))

(fn `Reset`
  (set `self.currGameTime` 0.0)
  (set `self.intervalTimer` 0.0)
  (set `self.currScore` 0))

(fn `SpawnBomb`
  (params (Position :type "Vector Structure"))
  (bind (_bombspawnchance _fallspeedmultiplier _spawninterval _bombdeductionscore _bombexplosionradius) (break `/Game/Lessons/Lesson3/miniProject3/Blueprints/Structs/S_DifficultySettings` (`self.currGameDetails`)))
  (bind _returnvalue (`|SpawnActorFromClass` "/Game/Lessons/Lesson3/miniProject3/Blueprints/BP_Bomb.BP_Bomb_C" (`KismetMathLibrary.MakeTransform` Position) "Undefined" "OverrideRootScale" null null))
  (`/Game/Lessons/Lesson3/miniProject3/Blueprints/BP_Bomb.OnCreate` _returnvalue _fallspeedmultiplier (`self.minHeight`) _bombexplosionradius _bombdeductionscore))

(fn `SpawnFruit`
  (params (Position :type "Vector Structure"))
  (bind _fruittype (`self.ChooseFruit`))
  (for _array_element (`self.possibleFruits`)
    (bind (_fruittype_2 _fruitmesh _fruitmeshscale) (break `/Game/Lessons/Lesson3/miniProject3/Blueprints/Structs/S_Fruit` _array_element))
    (if (`|EnumEquality` _fruittype _fruittype_2)
      (bind _returnvalue (`|SpawnActorFromClass` "/Game/Lessons/Lesson3/miniProject3/Blueprints/BP_Fruit.BP_Fruit_C" (`KismetMathLibrary.MakeTransform` Position (struct) _fruitmeshscale) "Undefined" "OverrideRootScale" null null))
      (`/Game/Lessons/Lesson3/miniProject3/Blueprints/BP_Fruit.OnCreate` _returnvalue _array_element (`.FallSpeedMultiplier_6_7BC1094BAC4909F2CC0CA38822C02611` (break `/Game/Lessons/Lesson3/miniProject3/Blueprints/Structs/S_DifficultySettings` (`self.currGameDetails`))) (`self.minHeight`))
      (break))))

(fn `SpawnObject`
  (params (location :type "Vector Structure"))
  (if (<= (`KismetMathLibrary.RandomFloatInRange` 0.0 1.0) (`.BombSpawnChance_2_2BD566AF0643C2FE6CAB41909AD4EDA7` (break `/Game/Lessons/Lesson3/miniProject3/Blueprints/Structs/S_DifficultySettings` (`self.currGameDetails`))))
    (`self.SpawnBomb` location)
    (else
      (`self.SpawnFruit` location))))

(fn `SpawnObstacles`
  (bind _returnvalue (`|SpawnActorFromClass` "/Game/Lessons/Lesson3/miniProject3/Blueprints/BP_Blocker.BP_Blocker_C" (`KismetMathLibrary.MakeTransform` (`self.obstacleOrigin`) (struct :`Yaw` 90.0)) "Undefined" "OverrideRootScale" null null))
  (set `self.obstacleInstance` _returnvalue))

(fn `StartGame`
  (params (GameNumber :type Integer))
  (bind _statustext (`self.statusText`))
  (bind _output_get (set `self.currentLevel` GameNumber))
  (set `self.currGameDetails` (`|GetArrayItem` (`self.allGameDetails`) _output_get))
  (set `self.inGame` true)
  (`self.Reset`)
  (`/Game/Lessons/Lesson3/miniProject3/Blueprints/BP_VisibilityManager.SetNotVisible` (`self.visibilityManager`))
  (bind _returnvalue (+ _output_get 1))
  (`/Game/Lessons/Lesson3/miniProject3/Blueprints/BP_Text.ShowText` (`self.scoreText`) (`|FormatText` "Level {level}<br>Current Score: 0<br>Highscore: {highscore}" _returnvalue (`|GetArrayItem` (`self.HighScores`) _output_get)))
  (`/Game/Lessons/Lesson3/miniProject3/Blueprints/BP_Text.ShowTextForSeconds` _statustext 2.0 "Game Start!")
  (`GameplayStatics.PlaySoundAtLocation` "/Game/Audio/SoundWaves/Drum/SW_ElectronicSnare.SW_ElectronicSnare" (`self.K2_GetActorLocation` _statustext) (struct) 1.0 1.0 0.0 null null null null)
  (if (== _returnvalue (`self.numGames`))
    (`self.SpawnObstacles`)))

(fn `UpdateGameEndStatus`
  (params (scoreUpdated :type Boolean))
  (bind _statustext (`self.statusText`))
  (bind _returnvalue (`self.K2_GetActorLocation` _statustext))
  (if (< (`self.currScore`) 0)
    (`/Game/Lessons/Lesson3/miniProject3/Blueprints/BP_Text.ShowTextForSeconds` _statustext 2.0 "Game End<br>Oh no! Negative score")
    (`GameplayStatics.PlaySoundAtLocation` "/Game/Audio/SoundWaves/Effect/SW_Laser_2.SW_Laser_2" _returnvalue (struct) 1.0 1.0 0.0 null null null null)
    (elif scoreUpdated
      (`/Game/Lessons/Lesson3/miniProject3/Blueprints/BP_Text.ShowTextForSeconds` _statustext 2.0 "Game End<br>New high score!")
      (`GameplayStatics.PlaySoundAtLocation` "/Game/Audio/SoundWaves/Effect/SW_Jump_3.SW_Jump_3" _returnvalue (struct) 1.0 1.0 0.0 null null null null)
      (else
        (`/Game/Lessons/Lesson3/miniProject3/Blueprints/BP_Text.ShowTextForSeconds` _statustext 2.0 "Game End")
        (`GameplayStatics.PlaySoundAtLocation` "/Game/Audio/SoundWaves/Effect/SW_Jump_2.SW_Jump_2" _returnvalue (struct) 1.0 1.0 0.0 null null null null)))))

(fn `UpdateHighScore`
  (returns (highscoreUpdated :type Boolean))
  (bind _highscores (`self.HighScores`))
  (bind _currscore (`self.currScore`))
  (bind _currentlevel (`self.currentLevel`))
  (if (> _currscore (`|GetArrayItem` _highscores _currentlevel))
    (`KismetArrayLibrary.Array_Set` _highscores _currentlevel _currscore)
    (return true)
    (else
      (return false))))

(fn `UpdateScore`
  (params (ChangeAmt :type Integer))
  (bind _currentlevel (`self.currentLevel`))
  (bind _output_get (set `self.currScore` (+ ChangeAmt (`self.currScore`))))
  (`/Game/Lessons/Lesson3/miniProject3/Blueprints/BP_Text.SetText` (`self.scoreText`) (`|FormatText` "Level {level}<br>Current Score: {score}<br>Highscore: {highscore}" (+ _currentlevel 1) _output_get (`|GetArrayItem` (`self.HighScores`) _currentlevel))))

(fn `UpdateTimers`
  (params (deltaSeconds :type "Float (double-precision)"))
  (set `self.currGameTime` (+ deltaSeconds (`self.currGameTime`)))
  (set `self.intervalTimer` (+ deltaSeconds (`self.intervalTimer`))))

(fn `UserConstructionScript`
  (bind _highscores (`self.HighScores`))
  (`KismetArrayLibrary.Array_Clear` _highscores)
  (for _ (range (+ (`self.numGames`) 1))
    (`KismetArrayLibrary.Array_Add` _highscores)
    (set `self.leftSpawnBound` (`self.K2_GetActorLocation` (`self.leftSpawnObj`)))
    (set `self.rightSpawnBound` (`self.K2_GetActorLocation` (`self.rightSpawnObj`)))
    (set `self.obstacleOrigin` (`self.K2_GetActorLocation` (`self.obstacleSpawnPoint`)))))