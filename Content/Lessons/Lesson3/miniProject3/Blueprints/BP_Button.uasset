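; Level-select button actor that starts its Level through BP_GameManager when interacted with.
; Its label shows the level number and high score from the manager, refreshed on BeginPlay and MakeVisible.
; The label starts hidden and follows a hover flag that Tick clears every frame, so it shows only while Hover keeps being called.
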(event `self.ReceiveBeginPlay`
  (bind _outactors (`GameplayStatics.GetAllActorsOfClass` "/Game/Lessons/Lesson3/miniProject3/Blueprints/BP_GameManager.BP_GameManager_C"))
  (set `self.gameManager` (`|GetArrayItem` _outactors))
  (`self.UpdateText`))

(event `self.ReceiveTick`
  (params (DeltaSeconds :type "Float (single-precision)"))
  (`self.UpdateTextVisibility` (`self.isHovered`))
  (set `self.isHovered` false))

(event `/Game/Lessons/Lesson3/miniProject3/Blueprints/Interfaces/BPI_Hoverable.Hover`
  (set `self.isHovered` true))

(event `/Game/Lessons/Lesson3/miniProject3/Blueprints/Interfaces/BPI_Interactable.Interact`
  (`/Game/Lessons/Lesson3/miniProject3/Blueprints/BP_GameManager.StartGame` (`self.gameManager`) (`self.level`)))

(fn `Make Visible`
  (`parent.Make Visible`)
  (`self.UpdateText`))

(fn `UpdateText`
  (bind _level (`self.level`))
  (bind _highscore (`/Game/Lessons/Lesson3/miniProject3/Blueprints/BP_GameManager.GetHighScore` (`self.gameManager`) _level))
  (`TextRenderComponent.K2_SetText` (`self.LevelText`) (`|FormatText` "Level {level}<br>Highscore: {highscore} " (+ _level 1) _highscore)))

(fn `UpdateTextVisibility`
  (params (NewVisibility :type Boolean))
  (`SceneComponent.SetVisibility` (`self.LevelText`) NewVisibility true))

(fn `UserConstructionScript`
  (`SceneComponent.SetVisibility` (`self.LevelText`) false false))