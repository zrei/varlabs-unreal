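; BP_CutFruitPiece is an actor for a piece of cut fruit that falls and spins until it is removed.
; OnCreate configures it with mesh, material, spin speed, fall direction, lifespan and minimum height.
; Tick moves it along that direction at a constant fall speed without sweeping, rolls it, and destroys it once it drops below the minimum height.
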(event `self.ReceiveBeginPlay`)

(event `self.ReceiveTick`
  (params (DeltaSeconds :type "Float (single-precision)"))
  (`self.Fall` DeltaSeconds)
  (`self.Rotate` DeltaSeconds)
  (`self.HeightCheck`))

(fn `Fall`
  (params (deltaSeconds :type "Float (double-precision)"))
  (`self.K2_AddActorWorldOffset` (* (* deltaSeconds (`self.fallSpeed`)) (`self.direction`))))

(fn `HeightCheck`
  (if (< (.z (`self.K2_GetActorLocation`)) (`self.minHeight`))
    (`self.K2_DestroyActor`)))

(fn `OnCreate`
  (params (Mesh :type "StaticMesh Object Reference") (Material :type "MaterialInstance Object Reference") (RotationalSpeed :type "Float (double-precision)") (FallDirection :type "Vector Structure") (Lifetime :type "Float (double-precision)") (minHeight :type "Float (double-precision)"))
  (bind _staticmesh (`self.StaticMesh`))
  (set `self.rotationalSpeed` RotationalSpeed)
  (`StaticMeshComponent.SetStaticMesh` _staticmesh Mesh)
  (`PrimitiveComponent.SetMaterial` _staticmesh 0 Material)
  (set `self.direction` FallDirection)
  (`self.SetLifeSpan` Lifetime)
  (set `self.minHeight` minHeight))

(fn `Rotate`
  (params (deltaSeconds :type "Float (double-precision)"))
  (`self.K2_AddActorWorldRotation` (`KismetMathLibrary.MakeRotator` (* (`self.rotationalSpeed`) deltaSeconds))))

(fn `UserConstructionScript`)