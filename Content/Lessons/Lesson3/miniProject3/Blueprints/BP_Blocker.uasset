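; BP_Blocker is a lesson mini-project actor that moves along a circular path around its starting location.
; On BeginPlay it prints a debug message, stores its origin and plays the Height timeline.
; Each update feeds the Circle track as degrees into cosine and sine, scaled by Radius, to set its position in the world YZ plane without sweeping.
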(event `self.ReceiveBeginPlay`
  (bind _radius (`self.Radius`))
  (`KismetSystemLibrary.PrintString` "Create Blocker")
  (bind _output_get (set `self.Origin` (`self.K2_GetActorLocation`)))
  (bind (_direction _circle) (`Timeline|Height` :!via `PlayFromStart`)
    (:`Update`
      (`self.K2_SetActorLocation` (+ (`KismetMathLibrary.MakeVector` 0.0 (* (`KismetMathLibrary.DegCos` _circle) _radius) (* (`KismetMathLibrary.DegSin` _circle) _radius)) _output_get)))))

(fn `UserConstructionScript`)