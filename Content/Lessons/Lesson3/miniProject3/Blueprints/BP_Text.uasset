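; BP_Text is an actor that shows in-world text messages through a text render component, starting hidden at BeginPlay.
; ShowText displays a string until it is hidden, while ShowTextForSeconds starts a timed display that Tick hides once the elapsed time exceeds the requested duration.
; The construction script applies the configurable font size as the text's world size.
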(event `self.ReceiveBeginPlay`
  (`self.Hide`))

(event `self.ReceiveTick`
  (params (DeltaSeconds :type "Float (single-precision)"))
  (if (`self.hideWithTime`)
    (bind _output_get (set `self.currTime` (+ DeltaSeconds (`self.currTime`))))
    (if (> _output_get (`self.timeToShow`))
      (`self.Hide`))))

(fn `Hide`
  (`SceneComponent.SetVisibility` (`self.Text`) false true))

(fn `SetText`
  (params (Text :type Text))
  (`TextRenderComponent.K2_SetText` (`self.Text`) Text))

(fn `Show`
  (`SceneComponent.SetVisibility` (`self.Text`) true true))

(fn `ShowText`
  (params (text :type Text))
  (set `self.hideWithTime` false)
  (`self.SetText` text)
  (`self.Show`))

(fn `ShowTextForSeconds`
  (params (time :type "Float (double-precision)") (text :type Text))
  (set `self.hideWithTime` true)
  (set `self.currTime` 0.0)
  (set `self.timeToShow` time)
  (`self.SetText` text)
  (`self.Show`))

(fn `UserConstructionScript`
  (`TextRenderComponent.SetWorldSize` (`self.Text`) (`self.fontSize`)))