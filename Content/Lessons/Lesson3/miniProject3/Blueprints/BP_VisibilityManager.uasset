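; BP_VisibilityManager is an actor that switches the visibility of all BP_VisibilityToggler actors in the level at once.
; On BeginPlay it caches every toggler into an Objects array.
; SetVisible and SetNotVisible store the state in an IsVisible flag and call MakeVisible or MakeNotVisible on each cached object.
; GetNotVisible returns the cached array only while IsVisible is false.
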(event `self.ReceiveBeginPlay`
  (bind _outactors (`GameplayStatics.GetAllActorsOfClass` "/Game/Lessons/Lesson3/miniProject3/Blueprints/BP_VisibilityToggler.BP_VisibilityToggler_C"))
  (set `self.Objects` _outactors))

(fn `GetNotVisible`
  (returns (NotVisibleObjects :type "Array of Actor Object Reference"))
  (if (`self.IsVisible`)
    (return)
    (else
      (return (`self.Objects`)))))

(fn `SetNotVisible`
  (set `self.IsVisible` false)
  (for _array_element (`self.Objects`)
    (`/Game/Lessons/Lesson3/miniProject3/Blueprints/BP_VisibilityToggler.Make Not Visible` _array_element)))

(fn `SetVisible`
  (set `self.IsVisible` true)
  (for _array_element (`self.Objects`)
    (`/Game/Lessons/Lesson3/miniProject3/Blueprints/BP_VisibilityToggler.Make Visible` _array_element)))

(fn `UserConstructionScript`)