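; BP_Fruit is a falling fruit actor that can be pushed away or cut for score.
; OnCreate applies mesh, material and fall speed from a fruit details struct.
; Tick moves it down until it drops below MinHeight and is destroyed, or along the push direction until its lifespan expires.
; Cut, ignored while pushed, spawns two opposed BP_CutFruitPiece halves, a BP_ScoreAddition and a chime, then destroys the fruit and returns its score.
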(event `self.ReceiveTick`
  (params (DeltaSeconds :type "Float (single-precision)"))
  (if (`self.isBeingPushed`)
    (`self.BePushed` DeltaSeconds)
    (else
      (`self.FallNormally` DeltaSeconds))))

(fn `BePushed`
  (params (deltaSeconds :type "Float (double-precision)"))
  (`self.K2_AddActorLocalOffset` (* (* deltaSeconds (`.PushSpeed_27_66BA6228E1444F177CB712B199742027` (break `/Game/Lessons/Lesson3/miniProject3/Blueprints/Structs/S_Fruit` (`self.fruitDetails`)))) (`self.pushDirection`))))

(fn `Cut`
  (returns (Score :type Integer))
  (bind (_fruittype _fruitmesh _fruitmeshscale _fruitcutpiecemesh _fruitcutpiecemeshscale _fruitmaterial _fruitcutmeshoffset _fruitcutmeshrotationalspeed _fruitcutmeshlifetime _pushlifespan _pushspeed _defaultfallspeed _score) (break `/Game/Lessons/Lesson3/miniProject3/Blueprints/Structs/S_Fruit` (`self.fruitDetails`)))
  (if (not (`self.isBeingPushed`))
    (`self.SpawnCutFruitPiece` _fruitcutmeshoffset (struct :`Roll` 90.0))
    (`self.SpawnCutFruitPiece` (`KismetMathLibrary.NegateVector` _fruitcutmeshoffset) (struct :`Roll` -90.0))
    (`|SpawnActorFromClass` "/Game/Lessons/Lesson3/BP_ScoreAddition.BP_ScoreAddition_C" (`KismetMathLibrary.MakeTransform` (`self.K2_GetActorLocation`)) "Undefined" "OverrideRootScale" null _score 20.0 null)
    (`GameplayStatics.SpawnSoundAtLocation` "/Game/Audio/SoundWaves/Effect/SW_Chime_1.SW_Chime_1" (0.0 0.0 0.0) (struct) 1.0 1.0 0.0 null null)
    (`self.K2_DestroyActor`)
    (return _score)))

(fn `FallNormally`
  (params (deltaSeconds :type "Float (double-precision)"))
  (bind _result (`/Engine/EditorBlueprintResources/StandardMacros.NegateFloat` (* deltaSeconds (`self.fallSpeed`)))
    (:`  `
      (`self.K2_AddActorLocalOffset` (`KismetMathLibrary.MakeVector` 0.0 0.0 _result))
      (if (< (.z (`self.K2_GetActorLocation`)) (`self.minHeight`))
        (`self.K2_DestroyActor`)))))

(fn `OnCreate`
  (params (Details :type "/Game/Lessons/Lesson3/miniProject3/Blueprints/Structs/S_Fruit Structure") (FallMultiplier :type "Float (double-precision)") (minHeight :type "Float (double-precision)"))
  (bind (_fruittype _fruitmesh _fruitmeshscale _fruitcutpiecemesh _fruitcutpiecemeshscale _fruitmaterial _fruitcutmeshoffset _fruitcutmeshrotationalspeed _fruitcutmeshlifetime _pushlifespan _pushspeed _defaultfallspeed) (break `/Game/Lessons/Lesson3/miniProject3/Blueprints/Structs/S_Fruit` Details))
  (`StaticMeshComponent.SetStaticMesh` (`self.StaticMesh`) _fruitmesh)
  (set `self.fallSpeed` (* _defaultfallspeed FallMultiplier))
  (`PrimitiveComponent.SetMaterial` (`self.StaticMesh`) 0 _fruitmaterial)
  (set `self.minHeight` minHeight)
  (set `self.fruitDetails` Details))

(fn `PushAway`
  (params (Direction :type "Vector Structure"))
  (set `self.pushDirection` Direction)
  (set `self.isBeingPushed` true)
  (`self.SetLifeSpan` (`.PushLifespan_30_3CFFC0401442778A8AED9086D6885BCE` (break `/Game/Lessons/Lesson3/miniProject3/Blueprints/Structs/S_Fruit` (`self.fruitDetails`)))))

(fn `SpawnCutFruitPiece`
  (params (Offset :type "Vector Structure") (Rotation :type "Rotator Structure"))
  (bind (_fruittype _fruitmesh _fruitmeshscale _fruitcutpiecemesh _fruitcutpiecemeshscale _fruitmaterial _fruitcutmeshoffset _fruitcutmeshrotationalspeed _fruitcutmeshlifetime) (break `/Game/Lessons/Lesson3/miniProject3/Blueprints/Structs/S_Fruit` (`self.fruitDetails`)))
  (bind _returnvalue (`|SpawnActorFromClass` "/Game/Lessons/Lesson3/miniProject3/Blueprints/BP_CutFruitPiece.BP_CutFruitPiece_C" (`KismetMathLibrary.MakeTransform` (+ Offset (`self.K2_GetActorLocation`)) Rotation (* (`self.GetActorScale3D`) _fruitcutpiecemeshscale)) "Undefined" "OverrideRootScale" null null))
  (`/Game/Lessons/Lesson3/miniProject3/Blueprints/BP_CutFruitPiece.OnCreate` _returnvalue _fruitcutpiecemesh _fruitmaterial _fruitcutmeshrotationalspeed (0.0 0.0 -1.0) _fruitcutmeshlifetime (`self.minHeight`)))

(fn `UserConstructionScript`)