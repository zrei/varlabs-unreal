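; BP_Bomb is a falling hazard that can be cut, exploding and returning a score deduction.
; OnCreate sets its fall speed, height limit, blast radius and deduction; Tick moves it vertically and destroys it below the limit.
; Cut fires only once, spawning a BP_ScoreAddition with the deduction before calling Explode.
; Explode uses a sphere overlap to push nearby BP_Fruit actors away, plays sound and particles, then destroys the bomb.
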(event `self.ReceiveTick`
  (params (DeltaSeconds :type "Float (single-precision)"))
  (`self.FallNormally` DeltaSeconds))

(fn `Cut`
  (returns (Score :type Integer))
  (bind _deductionscore (`self.DeductionScore`))
  (if (not (`self.hasExploded`))
    (set `self.hasExploded` true)
    (`|SpawnActorFromClass` "/Game/Lessons/Lesson3/BP_ScoreAddition.BP_ScoreAddition_C" (`KismetMathLibrary.MakeTransform` (`self.K2_GetActorLocation`)) "Undefined" "OverrideRootScale" null _deductionscore 20.0 null)
    (`self.Explode`)
    (return _deductionscore)))

(fn `Explode`
  (bind _returnvalue (`self.K2_GetActorLocation`))
  (bind (_outactors _returnvalue_2) (`KismetSystemLibrary.SphereOverlapActors` _returnvalue (`self.ExplosionRadius`) (`|MakeArray` "ObjectTypeQuery2" :!type "EObjectTypeQuery Enum") "/Game/Lessons/Lesson3/miniProject3/Blueprints/BP_Fruit.BP_Fruit_C"))
  (if _returnvalue_2
    (for _array_element _outactors
      (bind _asbp_fruit (cast `/Game/Lessons/Lesson3/miniProject3/Blueprints/BP_Fruit` _array_element))
      (`/Game/Lessons/Lesson3/miniProject3/Blueprints/BP_Fruit.PushAway` _asbp_fruit (`KismetMathLibrary.GetDirectionUnitVector` _returnvalue (`self.K2_GetActorLocation` _array_element))))
    (else
      (`KismetSystemLibrary.PrintString` "no collision")))
  (`GameplayStatics.PlaySoundAtLocation` "/Game/Audio/SoundWaves/Effect/SW_Explosion_3.SW_Explosion_3" _returnvalue (struct) 1.0 1.0 0.0 null null null null)
  (`GameplayStatics.SpawnEmitterAtLocation` "/Game/Effects/Particles/Explosion/P_NeonExplosion.P_NeonExplosion" _returnvalue)
  (`self.K2_DestroyActor`))

(fn `FallNormally`
  (params (deltaSeconds :type "Float (double-precision)"))
  (bind _result (`/Engine/EditorBlueprintResources/StandardMacros.NegateFloat` (* deltaSeconds (`self.currFallSpeed`)))
    (:`  `
      (`self.K2_AddActorLocalOffset` (`KismetMathLibrary.MakeVector` 0.0 0.0 _result))
      (if (< (.z (`self.K2_GetActorLocation`)) (`self.minHeight`))
        (`self.K2_DestroyActor`)))))

(fn `OnCreate`
  (params (fallSpeedMultiplier :type "Float (double-precision)") (minHeight :type "Float (double-precision)") (explosionRadius :type "Float (double-precision)") (deductionScore :type Integer))
  (set `self.currFallSpeed` (* fallSpeedMultiplier (`self.defaultFallSpeed`)))
  (set `self.minHeight` minHeight)
  (set `self.ExplosionRadius` explosionRadius)
  (set `self.DeductionScore` deductionScore))

(fn `UserConstructionScript`)