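; Gaze pointer that lets the player hover and interact with actors along the camera's forward line of sight.
; Every tick it line-traces from the camera, sends HoverMessage to the hit actor and moves a billboard reticle to the hit or ray end.
; The Act input retraces, sends InteractMessage and passes the target's CutMessage result to the GameManager's score.
; Traces ignore text actors and the VisibilityManager's non-visible actors, appended to the ignore list without clearing.
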(event `self.ReceiveTick`
  (params (DeltaSeconds :type "Float (single-precision)"))
  (`self.GetCameraRay`)
  (bind (_hashit _hitresult) (`self.RayTrace`))
  (bind (_bblockinghit _binitialoverlap _time _distance _location _impactpoint _normal _impactnormal _physmat _hitactor) (`GameplayStatics.BreakHitResult` _hitresult))
  (`self.GazeChecks` _hitactor _location _hashit (`self.rayEnd`)))

(event `self.ReceiveBeginPlay`
  (bind _outactors (`GameplayStatics.GetAllActorsOfClass` "/Game/Lessons/Lesson3/miniProject3/Blueprints/BP_VisibilityManager.BP_VisibilityManager_C"))
  (set `self.visibilityManager` (`|GetArrayItem` _outactors))
  (bind _outactors_2 (`GameplayStatics.GetAllActorsOfClass` "/Game/Lessons/Lesson3/miniProject3/Blueprints/BP_GameManager.BP_GameManager_C"))
  (set `self.gameManager` (`|GetArrayItem` _outactors_2))
  (bind _outactors_3 (`GameplayStatics.GetAllActorsOfClass` "/Game/Lessons/Lesson3/miniProject3/Blueprints/BP_Text.BP_Text_C"))
  (set `self.textObjects` _outactors_3))

(event `InputAction|Act`
  (params (Key :type "Key Structure"))
  (:`Pressed`
    (`self.GetCameraRay`)
    (bind (_hashit _hitresult) (`self.RayTrace`))
    (if _hashit
      (bind (_bblockinghit _binitialoverlap _time _distance _location _impactpoint _normal _impactnormal _physmat _hitactor) (`GameplayStatics.BreakHitResult` _hitresult))
      (`self.ClickChecks` _hitactor _location))))

(fn `ClickChecks`
  (params (HitObject :type "Actor Object Reference") (HitLocation :type "Vector Structure"))
  (message `/Game/Lessons/Lesson3/miniProject3/Blueprints/Interfaces/BPI_Interactable.Interact` HitObject)
  (bind _score (message `/Game/Lessons/Lesson3/miniProject3/Blueprints/Interfaces/BPI_Cuttable.Cut` HitObject))
  (`/Game/Lessons/Lesson3/miniProject3/Blueprints/BP_GameManager.UpdateScore` (`self.gameManager`) _score))

(fn `GazeChecks`
  (params (HitActor :type "Actor Object Reference") (HitLocation :type "Vector Structure") (HasHit :type Boolean) (NoHitLocation :type "Vector Structure"))
  (bind _materialbillboard (`self.MaterialBillboard`))
  (if HasHit
    (message `/Game/Lessons/Lesson3/miniProject3/Blueprints/Interfaces/BPI_Hoverable.Hover` HitActor)
    (`SceneComponent.K2_SetWorldLocation` _materialbillboard HitLocation false false)
    (else
      (`SceneComponent.K2_SetWorldLocation` _materialbillboard NoHitLocation false false))))

(fn `GetCameraRay`
  (bind _returnvalue (`GameplayStatics.GetPlayerCameraManager` 0))
  (bind _returnvalue_2 (`self.K2_GetActorLocation` _returnvalue))
  (set `self.rayStart` _returnvalue_2)
  (set `self.rayEnd` (+ (* (`self.GetActorForwardVector` _returnvalue) 10000.0) _returnvalue_2)))

(fn `RayTrace`
  (returns (HasHit :type Boolean) (HitResult :type "HitResult Structure"))
  (locals (itemsToIgnore :type "Array of Actor Object Reference"))
  (bind _notvisibleobjects (`/Game/Lessons/Lesson3/miniProject3/Blueprints/BP_VisibilityManager.GetNotVisible` (`self.visibilityManager`)))
  (`KismetArrayLibrary.Array_Append` (`local.itemsToIgnore`) _notvisibleobjects)
  (`KismetArrayLibrary.Array_Append` (`local.itemsToIgnore`) (`self.textObjects`))
  (bind (_outhit _returnvalue) (`KismetSystemLibrary.LineTraceSingle` (`self.rayStart`) (`self.rayEnd`) "TraceTypeQuery1" false (`local.itemsToIgnore`)))
  (return _returnvalue _outhit))

(fn `UserConstructionScript`)