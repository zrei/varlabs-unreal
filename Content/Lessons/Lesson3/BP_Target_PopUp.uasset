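; Pop-up target actor that moves vertically and can be destroyed through interaction.
; On BeginPlay it stores its origin, waits a random delay to stagger its start, then plays the UpAndDown timeline to offset its height from that origin, printing the value each update.
; Interact prints a message, spawns a small neon explosion, destroys the actor and returns a fixed integer.
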(event `self.ReceiveBeginPlay`
  (bind _output_get (set `self.Origin` (`self.K2_GetActorLocation`)))
  (`KismetSystemLibrary.Delay` (`KismetMathLibrary.RandomFloatInRange` 0.0 5.0))
  (bind (_direction _data) (`Timeline|UpAndDown` :!via `PlayFromStart`)
    (:`Update`
      (`KismetSystemLibrary.PrintString` (`KismetStringLibrary.Conv_DoubleToString` _data))
      (`self.K2_SetActorLocation` (+ _output_get (* _data (0.0 0.0 20.0)))))))

(fn `Interact`
  (returns (Score :type Integer))
  (`KismetSystemLibrary.PrintString` "Interaction")
  (`GameplayStatics.SpawnEmitterAtLocation` "/Game/Effects/Particles/Explosion/P_NeonExplosion_Tiny.P_NeonExplosion_Tiny" (`self.K2_GetActorLocation`))
  (`self.K2_DestroyActor`)
  (return 5))

(fn `UserConstructionScript`)