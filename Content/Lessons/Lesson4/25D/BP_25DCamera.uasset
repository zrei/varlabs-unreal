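; BP_25DCamera is a camera actor for a 2.5D lesson that follows the player character along Y and Z.
; On BeginPlay it stores its own X location and its offset from the player.
; Every Tick it combines the stored X with the player's current Y and Z, adds the full offset (X included), and moves there directly, without smoothing or sweep.
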(event `self.ReceiveBeginPlay`
  (bind _returnvalue (`self.K2_GetActorLocation`))
  (set `self.CameraXLocation` (.x _returnvalue))
  (set `self.CameraOffset` (- _returnvalue (`self.K2_GetActorLocation` (`GameplayStatics.GetPlayerCharacter` 0)))))

(event `self.ReceiveTick`
  (params (DeltaSeconds :type "Float (single-precision)"))
  (bind (_returnvalue_x _returnvalue_y _returnvalue_z) (`KismetMathLibrary.BreakVector` (`self.K2_GetActorLocation` (`GameplayStatics.GetPlayerCharacter` 0))))
  (`self.K2_SetActorLocation` (+ (`KismetMathLibrary.MakeVector` (`self.CameraXLocation`) _returnvalue_y _returnvalue_z) (`self.CameraOffset`))))

(fn `UserConstructionScript`)