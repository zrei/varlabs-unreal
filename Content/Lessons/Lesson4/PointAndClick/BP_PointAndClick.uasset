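; BP_PointAndClick is a player character for a lesson on point-and-click teleport movement with stepped VR-style turning.
; Each tick, mouse movement drives a BPCMouseCursor component, which turns green or red depending on whether the traced hit is walkable.
; The Teleport action moves the character to a valid cursor location, offset by capsule half-height.
; Holding right mouse freezes the cursor and accumulates Turn input into fixed-angle snap turns.
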(event `self.ReceiveTick`
  (params (DeltaSeconds :type "Float (single-precision)"))
  (bind (_deltax _deltay) (`PlayerController.GetInputMouseDelta` (`GameplayStatics.GetPlayerController` 0)))
  (if (not (`self.CanTurn`))
    (bind _tracehit (`/Game/Blueprints/Utility/BPC_MouseCursor.Update` (`self.BPC_MouseCursor`) (/ _deltax 3.0) (/ _deltay 3.0)))
    (bind _output_get (set `self.CanTeleport` (`CharacterMovementComponent.IsWalkable` (`self.CharacterMovement`) _tracehit)))
    (if _output_get
      (`/Game/Blueprints/Utility/BPC_MouseCursor.SetCursorColor` (`self.BPC_MouseCursor`) (struct :`R` 0.401166 :`G` 1.0 :`B` 0.531252 :`A` 1.0))
      (else
        (`/Game/Blueprints/Utility/BPC_MouseCursor.SetCursorColor` (`self.BPC_MouseCursor`) (struct :`R` 1.0 :`A` 1.0))))))

(event `Key|RightMouseButton`
  (params (Key :type "Key Structure"))
  (:`Pressed`
    (set `self.CanTurn` true))
  (:`Released`
    (set `self.CanTurn` false)))

(event `InputAction|Teleport`
  (params (Key :type "Key Structure"))
  (:`Pressed`
    (if (`self.CanTeleport`)
      (`self.K2_SetActorLocation` (+ (`/Game/Blueprints/Utility/BPC_MouseCursor.GetCursorLocation` (`self.BPC_MouseCursor`)) (`KismetMathLibrary.MakeVector` 0.0 0.0 (`CapsuleComponent.GetScaledCapsuleHalfHeight` (`self.CapsuleComponent`))))))))

(event `InputAxis|Turn`
  (params (AxisValue :type "Float (single-precision)"))
  (if (`self.CanTurn`)
    (bind _output_get (set `self.TurnMouseDelta` (+ AxisValue (`self.TurnMouseDelta`))))
    (if (> _output_get 5.0)
      (`/Game/Blueprints/Utility/VARlabsVRUtilityFunctions.Turn VR Player` 20.0)
      (set `self.TurnMouseDelta` 0.0 :!label _label)
      (elif (< _output_get -5.0)
        (`/Game/Blueprints/Utility/VARlabsVRUtilityFunctions.Turn VR Player` -20.0)
        (goto _label)))))

(fn `UserConstructionScript`)