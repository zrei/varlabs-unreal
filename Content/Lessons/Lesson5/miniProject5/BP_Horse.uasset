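; BP_Horse is a horse actor built from static mesh parts that can either stay static or simulate physics.
; The construction script collects static mesh children of the root into Parts, and ActivatePhysics enables simulation on each.
; OnCreate sets IsStatic and activates physics immediately for non-static horses; actor overlap also activates it if not already active.
; A swept falling movement using InitialFallSpeed exists but is disconnected and never runs.
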(event `self.ReceiveActorBeginOverlap`
  (params (OtherActor :type "Actor Object Reference"))
  (if (not (or (`self.IsStatic`) (`self.PhysicsActivated`)))
    (`self.ActivatePhysics`)))

(event `self.ReceiveTick`
  (params (DeltaSeconds :type "Float (single-precision)")))

(fn `ActivatePhysics`
  (for _array_element (`self.Parts`)
    (`PrimitiveComponent.SetSimulatePhysics` _array_element true))
  (set `self.PhysicsActivated` true))

(fn `AddBodyPart`
  (params (BodyPart :type "StaticMeshComponent Object Reference"))
  (`KismetArrayLibrary.Array_Add` (`self.Parts`) BodyPart))

(fn `OnCreate`
  (params (IsStatic :type Boolean))
  (bind _output_get (set `self.IsStatic` IsStatic))
  (if (not _output_get)
    (`self.ActivatePhysics`)))

(fn `UserConstructionScript`
  (for _array_element (`SceneComponent.GetChildrenComponents` (`self.DefaultSceneRoot`) false)
    (bind _asstatic_mesh_component (cast `StaticMeshComponent` _array_element))
    (`self.AddBodyPart` _asstatic_mesh_component)))