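; BP_Domino is a domino actor that picks a random mesh from DominoMeshes on BeginPlay and topples when something overlaps it.
; The first overlap with anything other than a BP_Wall sets a one-time HasFallen flag, starts the fall and plays a thud sound.
; Tick animates the fall by adding local roll scaled by RotationalSpeed and delta time until the roll reaches -90 degrees or lower.
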(event `self.ReceiveBeginPlay`
  (`StaticMeshComponent.SetStaticMesh` (`self.Domino`) (`KismetArrayLibrary.Array_Random` (`self.DominoMeshes`))))

(event `self.ReceiveActorBeginOverlap`
  (params (OtherActor :type "Actor Object Reference"))
  (if (not (`self.hasFallen`))
    (cast `/Game/Lessons/Lesson2/miniProject2/Blueprints/BP_Wall` OtherActor
      (:`CastFailed`
        (set `self.hasFallen` true)
        (set `self.beginFalling` true)
        (`GameplayStatics.PlaySoundAtLocation` "/Game/Audio/SoundWaves/Effect/SW_Thud_1.SW_Thud_1" (`self.K2_GetActorLocation`) (struct) 1.0 1.0 0.0 null null null null)))))

(event `self.ReceiveTick`
  (params (DeltaSeconds :type "Float (single-precision)"))
  (if (`self.beginFalling`)
    (bind _result (`/Engine/EditorBlueprintResources/StandardMacros.NegateFloat` (* (`self.rotationalSpeed`) DeltaSeconds))
      (:`  `
        (`self.K2_AddActorLocalRotation` (`KismetMathLibrary.MakeRotator` _result))
        (if (<= (.roll (`self.K2_GetActorRotation`)) -90.0)
          (set `self.beginFalling` false))))))

(fn `UserConstructionScript`)