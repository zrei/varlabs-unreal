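; BP_Car is a car actor that circles a reference actor on a configurable, tiltable orbit.
; BeginPlay gives both body meshes one random material from a list, and Tick advances the angle by rotational speed.
; RotateAroundPoint spins a radius vector around Z, tilts it by the axis settings, adds the origin and orients the car.
; The construction script clamps the axis inputs and, given a valid reference, derives the origin and positions the car.
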(event `self.ReceiveBeginPlay`
  (bind _output_get (set `self.carMaterial` (`KismetArrayLibrary.Array_Random` (`self.Materials`))))
  (`PrimitiveComponent.SetMaterial` (`self.CarBodyBottom`) 0 _output_get)
  (`PrimitiveComponent.SetMaterial` (`self.CarBodyTop`) 0 _output_get))

(event `self.ReceiveTick`
  (params (DeltaSeconds :type "Float (single-precision)"))
  (set `self.angularRot` (+ (* (`self.RotationalSpeed`) DeltaSeconds) (`self.angularRot`)))
  (`self.RotateAroundPoint`))

(fn `RotateAroundPoint`
  (bind _yrot (`self.yRot`))
  (bind _axisrot (`self.axisRot`))
  (bind _angularrot (`self.angularRot`))
  (bind _xrot (`self.xRot`))
  (`self.K2_SetActorLocation` (+ (`KismetMathLibrary.RotateAngleAxis` (`KismetMathLibrary.RotateAngleAxis` (* (`self.Radius`) (1.0 0.0 0.0)) _angularrot (0.0 0.0 1.0)) _axisrot (`KismetMathLibrary.MakeVector` _xrot _yrot)) (`self.Origin`)))
  (`self.K2_SetActorRotation` (`KismetMathLibrary.RotatorFromAxisAndAngle` (`KismetMathLibrary.MakeVector` _xrot _yrot 1.0) _axisrot))
  (`self.K2_AddActorLocalRotation` (`KismetMathLibrary.MakeRotator` 0.0 -90.0 _angularrot)))

(fn `UserConstructionScript`
  (bind _originreference (`self.OriginReference`))
  (`self.ValidateAxisValues`)
  (if (`KismetSystemLibrary.IsValid` _originreference)
    (set `self.Origin` (+ (`self.K2_GetActorLocation` _originreference) (`self.Offset`)))
    (`self.RotateAroundPoint`)))

(fn `ValidateAxisValues`
  (set `self.xRot` (`KismetMathLibrary.FClamp` (`self.xRot`) -1.0))
  (set `self.yRot` (`KismetMathLibrary.FClamp` (`self.yRot`) -1.0)))