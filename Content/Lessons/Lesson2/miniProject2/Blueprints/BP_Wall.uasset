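; BP_Wall is a configurable wall actor from a lesson mini-project that sets up its appearance in the Construction Script.
; It assigns the Model mesh to its StaticMesh component.
; When OverrideMaterials is enabled, it loops over every material slot and applies NewMaterial to each.
; The event graph holds only disabled placeholder events, so it has no runtime logic.
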(fn `UserConstructionScript`
  (`StaticMeshComponent.SetStaticMesh` (`self.StaticMesh`) (`self.Model`))
  (if (`self.OverrideMaterials`)
    (for _index (range (`PrimitiveComponent.GetNumMaterials` (`self.StaticMesh`)))
      (`PrimitiveComponent.SetMaterial` (`self.StaticMesh`) _index (`self.NewMaterial`)))))