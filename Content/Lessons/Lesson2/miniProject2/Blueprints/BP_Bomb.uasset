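; BP_Bomb is a projectile actor that flies in a straight line and explodes on impact or when its lifetime runs out.
; OnCreate takes a target location, stores the direction toward it and adds the look-at rotation, while Tick moves the bomb with a swept offset scaled by Speed.
; Overlaps with anything except other bombs or Pawns, or expiry of the Life delay, call OnDestroy, which plays explosion sound and particles before destroying the actor.
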(event `self.ReceiveBeginPlay`
  (`KismetSystemLibrary.Delay` (`self.Life`))
  (`self.OnDestroy`))

(event `self.ReceiveActorBeginOverlap`
  (params (OtherActor :type "Actor Object Reference"))
  (cast `/Game/Lessons/Lesson2/miniProject2/Blueprints/BP_Bomb` OtherActor
    (:`CastFailed`
      (cast `Pawn` OtherActor
        (:`CastFailed`
          (`KismetSystemLibrary.PrintString` "Collision Destroy")
          (`self.OnDestroy`))))))

(event `self.ReceiveTick`
  (params (DeltaSeconds :type "Float (single-precision)"))
  (`self.K2_AddActorWorldOffset` (* (`self.UnitDirection`) (* DeltaSeconds (`self.Speed`))) true))

(fn `OnCreate`
  (params (Target :type "Vector Structure"))
  (bind _returnvalue (`self.K2_GetActorLocation`))
  (set `self.UnitDirection` (`KismetMathLibrary.GetDirectionUnitVector` _returnvalue Target))
  (`self.K2_AddActorWorldRotation` (`KismetMathLibrary.FindLookAtRotation` _returnvalue Target)))

(fn `OnDestroy`
  (bind _returnvalue (`self.K2_GetActorLocation`))
  (`GameplayStatics.PlaySoundAtLocation` "/Game/Audio/SoundWaves/Effect/SW_Explosion_3.SW_Explosion_3" _returnvalue (struct) 1.0 1.0 0.0 null null null null)
  (`GameplayStatics.SpawnEmitterAtLocation` "/Game/Effects/Particles/Explosion/P_AsteroidExplosion.P_AsteroidExplosion" _returnvalue)
  (`self.K2_DestroyActor`))

(fn `UserConstructionScript`)