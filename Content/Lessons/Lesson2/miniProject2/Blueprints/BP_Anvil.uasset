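; BP_Anvil is a falling anvil actor from a lesson mini-project that plays a sound at its location when it spawns.
; Tick moves it along world Z by FallSpeed scaled by delta time, using a swept offset.
; On overlap it destroys itself unless the other actor matches BP_Wall or is a Pawn, and pawn overlaps trigger no action here.
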(event `self.ReceiveBeginPlay`
  (`GameplayStatics.PlaySoundAtLocation` "/Game/Audio/SoundWaves/Effect/SW_Jump_3.SW_Jump_3" (`self.K2_GetActorLocation`) (struct) 1.0 1.0 0.0 null null null null))

(event `self.ReceiveActorBeginOverlap`
  (params (OtherActor :type "Actor Object Reference"))
  (if (not (== OtherActor "/Game/Lessons/Lesson2/miniProject2/Blueprints/BP_Wall.BP_Wall"))
    (cast `Pawn` OtherActor
      (:`CastFailed`
        (`self.K2_DestroyActor`)))))

(event `self.ReceiveTick`
  (params (DeltaSeconds :type "Float (single-precision)"))
  (bind _result (`/Engine/EditorBlueprintResources/StandardMacros.NegateFloat` (* (`self.Fall Speed`) DeltaSeconds))
    (:`  `
      (`self.K2_AddActorWorldOffset` (`KismetMathLibrary.MakeVector` 0.0 0.0 _result) true))))

(fn `UserConstructionScript`)